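; Ball actor for a brick-breaker game that bounces between the player, bricks and static meshes, scoring brick hits.
; While Moving, Tick sweeps it along Velocity at a capped per-frame step that grows with level, randomizing downward Velocity when zero.
; Sphere hits flip Z off the player, or Z or Y by normal otherwise, except bricks reduced to zero HitValue.
; Non-player hits also trigger NextLevel when no bricks remain.
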(event `self.ReceiveBeginPlay`
  (bind _asplayer_character (cast `/Game/basicSetup/PlayerCharacter` (`GameplayStatics.GetPlayerPawn` 0)))
  (set `self.char` _asplayer_character))

(event `self.ReceiveTick`
  (params (DeltaSeconds :type "Float (single-precision)"))
  (bind _velocity (`self.velocity`))
  (bind _returnvalue (+ (* (`/Game/basicSetup/PlayerCharacter.level` (`self.char`)) 0.125) 3.875))
  (bind _returnvalue_2 (`KismetMathLibrary.SelectFloat` _returnvalue 15.0 (<= _returnvalue 15.0)))
  (if (`self.moving`)
    (if (> (`KismetMathLibrary.VSize` _velocity) 0.0)
      (`self.K2_SetActorLocation` (+ (`self.K2_GetActorLocation`) (* _velocity _returnvalue_2)) true)
      (else
        (bind _output_get (set `self.velocity` (`KismetMathLibrary.MakeVector` 0.0 (`KismetMathLibrary.RandomFloatInRange` -1.0 1.0) -1.0)))
        (`self.K2_SetActorLocation` (+ (`self.K2_GetActorLocation`) (* _output_get _returnvalue_2)) true)))))

(event `self.Sphere.OnComponentHit`
  (params (HitComponent :type "PrimitiveComponent Object Reference") (OtherActor :type "Actor Object Reference") (OtherComp :type "PrimitiveComponent Object Reference") (NormalImpulse :type "Vector Structure") (Hit :type "HitResult Structure (by ref)"))
  (bind (_bblockinghit _binitialoverlap _time _location _impactpoint _normal _impactnormal _physmat _hitactor) (`GameplayStatics.BreakHitResult` Hit))
  (bind _char (`self.char`))
  (bind _char_2 (`self.char`))
  (if (== _hitactor (`self.char`))
    (set `self.velocity` (`KismetMathLibrary.MakeVector` (.x (`self.velocity`)) (.y (`self.velocity`)) (* (.z (`self.velocity`)) -1.0)))
    (else
      (bind _outactors (`GameplayStatics.GetAllActorsOfClass` "/Game/Blueprints/BP_brick.BP_brick_C"))
      (for _array_element _outactors
        (if (== _hitactor _array_element)
          (set `/Game/basicSetup/PlayerCharacter.score` (+ (`/Game/basicSetup/PlayerCharacter.score` _char_2) 10) _char_2)
          (bind _hitvalue (`/Game/Blueprints/BP_brick.hitValue` _array_element))
          (`/Engine/EditorBlueprintResources/StandardMacros.DecrementInt` _hitvalue
            (:`  `
              (if (== _hitvalue 0)
                (break)
                (elif (!= (.z _normal) 0.0)
                  (set `self.velocity` (`KismetMathLibrary.MakeVector` (.x (`self.velocity`)) (.y (`self.velocity`)) (* (.z (`self.velocity`)) -1.0)))
                  (break)
                  (elif (!= (.y _normal) 0.0)
                    (set `self.velocity` (`KismetMathLibrary.MakeVector` (.x (`self.velocity`)) (* (.y (`self.velocity`)) -1.0) (.z (`self.velocity`))))
                    (break)
                    (else
                      (break)))))))))
      (bind _outactors_2 (`GameplayStatics.GetAllActorsOfClass` "/Script/Engine.StaticMeshActor"))
      (for _array_element_2 _outactors_2
        (if (== _array_element_2 _hitactor)
          (if (!= (.z _normal) 0.0)
            (set `self.velocity` (`KismetMathLibrary.MakeVector` (.x (`self.velocity`)) (.y (`self.velocity`)) (* (.z (`self.velocity`)) -1.0)))
            (break)
            (elif (!= (.y _normal) 0.0)
              (set `self.velocity` (`KismetMathLibrary.MakeVector` (.x (`self.velocity`)) (* (.y (`self.velocity`)) -1.0) (.z (`self.velocity`))))
              (break)
              (else
                (break))))))
      (if (< (`/Game/basicSetup/PlayerCharacter.numBricks` _char) 1)
        (`/Game/basicSetup/PlayerCharacter.NextLevel` _char)))))

(fn `UserConstructionScript`)