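; BP_brick is a brick actor whose look reflects its remaining HitValue, likely for a brick-breaker game.
; Every Tick it sets the mesh material: a hex tile for BlockBrick, otherwise copper, chrome or gold by HitValue.
; When a non-block brick's HitValue is zero, it decrements NumBricks on the PlayerCharacter and destroys itself.
; HitValue is only read here, never changed.
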(event `self.ReceiveTick`
  (params (DeltaSeconds :type "Float (single-precision)"))
  (bind _brick (`self.Brick`))
  (if (`self.BlockBrick`)
    (`PrimitiveComponent.SetMaterial` _brick 0 "/Game/MobileStarterContent/Materials/M_Tech_Hex_Tile.M_Tech_Hex_Tile")
    (else
      (switch `int` (`self.hitValue`)
        (:`Default`
          _)
        (:`1`
          (`PrimitiveComponent.SetMaterial` _brick 0 "/Game/MobileStarterContent/Materials/M_Metal_Copper.M_Metal_Copper"))
        (:`2`
          (`PrimitiveComponent.SetMaterial` _brick 0 "/Game/MobileStarterContent/Materials/M_Metal_Chrome.M_Metal_Chrome"))
        (:`3`
          (`PrimitiveComponent.SetMaterial` _brick 0 "/Game/MobileStarterContent/Materials/M_Metal_Gold.M_Metal_Gold")))
      (if (== (`self.hitValue`) 0)
        (bind _asplayer_character (cast `/Game/basicSetup/PlayerCharacter` (`GameplayStatics.GetPlayerPawn` 0)))
        (`/Engine/EditorBlueprintResources/StandardMacros.DecrementInt` (`/Game/basicSetup/PlayerCharacter.numBricks` _asplayer_character)
          (:`  `
            (`self.K2_DestroyActor`)))))))

(fn `UserConstructionScript`)